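; Spear trap actor that periodically thrusts a spear mesh upward and damages the third-person player character.
; After an initial delay on BeginPlay, a looping timer replays a timeline each cycle, lerping the mesh's relative Z from zero to a configurable pop-up height.
; A separate damage box applies damage to BP_ThirdPersonCharacter on begin overlap, with no check on the timeline's state.
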(event `self.ReceiveBeginPlay`
  (`KismetSystemLibrary.Delay` (`self.InitialDelay`))
  (`KismetSystemLibrary.K2_SetTimerDelegate` (delegate `TriggerTrap`) (`self.CycleInterval`) true))

(event `TriggerTrap`
  (bind (_direction _alpha) (`Timeline|TL_SpikeMove` :!via `PlayFromStart`)
    (:`Update`
      (`SceneComponent.K2_SetRelativeLocation` (`self.SpearMesh`) (`KismetMathLibrary.MakeVector` 0.0 0.0 (`KismetMathLibrary.Lerp` 0.0 (`self.PopUpHeight`) _alpha)) false false))))

(event `self.DamegeBox.OnComponentBeginOverlap`
  (params (OverlappedComponent :type "PrimitiveComponent Object Reference") (OtherActor :type "Actor Object Reference") (OtherComp :type "PrimitiveComponent Object Reference") (OtherBodyIndex :type Integer) (bFromSweep :type Boolean) (SweepResult :type "HitResult Structure (by ref)"))
  (bind _asbp_third_person_character (cast `/Game/ThirdPerson/Blueprints/BP_ThirdPersonCharacter` OtherActor))
  (`GameplayStatics.ApplyDamage` _asbp_third_person_character 1.0))

(fn `UserConstructionScript`)