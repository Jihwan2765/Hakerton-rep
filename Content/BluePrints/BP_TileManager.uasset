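; BP_TileManager is a Blueprint that drops the level's BP_Tile actors one at a time, in ascending order of X location.
; On BeginPlay it gathers all BP_Tile actors into RemainingTiles and waits StartDelay before starting.
; DropNextTile linearly searches for the lowest-X tile, calls its DropTile, removes it, and calls itself again after DropInterval until none remain.
; The SortTilesByX function is an empty stub.
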(event `self.ReceiveBeginPlay`
  (bind _outactors (`GameplayStatics.GetAllActorsOfClass` "/Game/BluePrints/BP_Tile.BP_Tile_C"))
  (set `self.RemainingTiles` _outactors)
  (`KismetSystemLibrary.Delay` (`self.StartDelay`))
  (`self.DropNextTile`))

(event `DropNextTile`
  (bind _besttile (`self.BestTile`))
  ; 초기 세팅
  (if (> (`KismetArrayLibrary.Array_Length` (`self.RemainingTiles`)) 0)
    (bind _output_get (set `self.BestTile` (`|GetArrayItem` (`self.RemainingTiles`))))
    (bind _returnvalue_x (`KismetMathLibrary.BreakVector` (`self.K2_GetActorLocation` _output_get)))
    (set `self.BestX` _returnvalue_x)
    ; Best 타일 찾기 알고리즘
    (for _index (range 1 (`KismetArrayLibrary.Array_Length` (`self.RemainingTiles`)))
      (bind _output (`|GetArrayItem` (`self.RemainingTiles`) _index))
      (bind _returnvalue_x_2 (`KismetMathLibrary.BreakVector` (`self.K2_GetActorLocation` _output)))
      (if (< _returnvalue_x_2 (`self.BestX`))
        (set `self.BestTile` _output)
        (set `self.BestX` _returnvalue_x_2)))
    ; Best타일 Drop하고 배열에서 삭제
    (`/Game/BluePrints/BP_Tile.DropTile` _besttile)
    (`KismetArrayLibrary.Array_RemoveItem` (`self.RemainingTiles`) _besttile)
    (`KismetSystemLibrary.Delay` (`self.DropInterval`))
    (`self.DropNextTile`)))

(fn `SortTilesByX`)

(fn `UserConstructionScript`)